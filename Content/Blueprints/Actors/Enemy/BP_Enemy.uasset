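; Enemy actor Blueprint that travels along the path of a referenced EnemySpline, starting on BeginPlay.
; A timeline's play rate is set from TimeToComplete, so that variable controls how long the trip takes.
; Each update lerps the timeline's alpha over the spline length and sets the actor's world location and rotation at that distance.
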(event `self.ReceiveBeginPlay`
  (`self.MoveEnemy`))

(event `MoveEnemy`
  (bind _enemysplinepath (`EnemySplinePath.EnemySplinePath` (`self.Enemy Spline`)))
  (`TimelineComponent.SetPlayRate` (`self.EnemyMove`) (/ 1.0 (`self.Time To Complete`)))
  (bind (_direction _move_track) (`Timeline|EnemyMove`)
    (:`Update`
      (bind _returnvalue (`KismetMathLibrary.Lerp` 0.0 (`SplineComponent.GetSplineLength` _enemysplinepath) _move_track))
      (`self.K2_SetActorLocationAndRotation` (`SplineComponent.GetLocationAtDistanceAlongSpline` _enemysplinepath _returnvalue "World") (`SplineComponent.GetRotationAtDistanceAlongSpline` _enemysplinepath _returnvalue "World")))))

(fn `UserConstructionScript`)